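; BP_Building is a building actor that constructs itself over time by rising from its starting height.
; BeginPlay caches the Building component's relative Z as the baseline.
; Until built or ruined, Tick advances Progress by BuildingVelocity, raises the component proportionally to Height and shows the percentage on BuildingStatus.
; At full progress it sets IsBuilt and hides the status text; the built-and-ruined branch is empty.
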(event `self.ReceiveBeginPlay`
  (set `self.originalZ` (.z (`SceneComponent.RelativeLocation` (`self.Building`)))))

(event `self.ReceiveTick`
  (params (DeltaSeconds :type "Float (single-precision)"))
  (bind _isruined (`self.isRuined`))
  (bind _building (`self.Building`))
  (bind _progress (`self.progress`))
  (bind _returnvalue (+ _progress (* DeltaSeconds (`self.buildingVelocity`))))
  (if (`self.isBuilt`)
    (if _isruined
      _)
    (elif (not _isruined)
      (`/Engine/EditorBlueprintResources/StandardMacros.CompareFloat` _progress 100.0
        (:`>`
          (set `self.isBuilt` true :!label _label)
          (`SceneComponent.SetHiddenInGame` (`self.BuildingStatus`) true false))
        (:`==`
          (goto _label))
        (:`<`
          (bind _output_get (set `self.progress` _returnvalue))
          (`SceneComponent.K2_SetRelativeLocation` _building (`KismetMathLibrary.MakeVector` (.x (`SceneComponent.RelativeLocation` _building)) (.y (`SceneComponent.RelativeLocation` _building)) (+ (`self.originalZ`) (* (/ _returnvalue 100.0) (`self.height`)))) false false)
          (`TextRenderComponent.K2_SetText` (`self.BuildingStatus`) (`KismetTextLibrary.Conv_StringToText` (`KismetStringLibrary.Concat_StrStr` (`KismetStringLibrary.Conv_IntToString` (`KismetMathLibrary.FTrunc` _output_get)) "%"))))))))

(fn `UserConstructionScript`)