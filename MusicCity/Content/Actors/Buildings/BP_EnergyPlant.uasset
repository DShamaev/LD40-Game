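; Energy plant building actor that costs the player craft resources to build.
; CheckIfCouldBeBuild reports whether the TopDownController's CraftRes covers RequiredCM.
; On BeginPlay it deducts that cost from the controller directly, without repeating the check.
; The UpdateResourcesforPlayer event calls EnergyPlantDidBuilt on the controller to signal that the plant is built.
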(event `self.ReceiveBeginPlay`
  (bind _astop_down_controller (cast `/Game/Gameplay/TopDownController` (`GameplayStatics.GetPlayerController` 0)))
  (set `/Game/Gameplay/TopDownController.craftRes` (- (`/Game/Gameplay/TopDownController.craftRes` _astop_down_controller) (`self.requiredCM`)) _astop_down_controller))

(event `self.UpdateResourcesForPlayer`
  (bind _astop_down_controller (cast `/Game/Gameplay/TopDownController` (`GameplayStatics.GetPlayerController` 0)))
  (`/Game/Gameplay/TopDownController.energyPlantDidBuilt` _astop_down_controller))

(fn `CheckIfCouldBeBuild`
  (returns (couldBeBuilt :type Boolean))
  (bind _astop_down_controller (cast `/Game/Gameplay/TopDownController` (`GameplayStatics.GetPlayerController` 0)))
  (`/Engine/EditorBlueprintResources/StandardMacros.CompareInt` (- (`/Game/Gameplay/TopDownController.craftRes` _astop_down_controller) (`self.requiredCM`))
    (:`>`
      _)
    (:`==`
      _)
    (:`<`
      (return false)))
  (return true))

(fn `UserConstructionScript`)