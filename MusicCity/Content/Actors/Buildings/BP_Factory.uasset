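; Factory building actor that charges the player a crafting resource and energy cost when it spawns.
; BeginPlay subtracts the required amounts from the TopDownController of player 0, flooring each balance at zero.
; CheckIfCouldBeBuild reports whether that controller can afford both costs.
; A separate UpdateResourcesforPlayer event notifies the controller through FactoryDidBuild.
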(event `self.ReceiveBeginPlay`
  (bind _astop_down_controller (cast `/Game/Gameplay/TopDownController` (`GameplayStatics.GetPlayerController` 0)))
  (bind _returnvalue (- (`/Game/Gameplay/TopDownController.craftRes` _astop_down_controller) (`self.requiredCM`)))
  (`/Engine/EditorBlueprintResources/StandardMacros.CompareInt` _returnvalue
    (:`>`
      (set `/Game/Gameplay/TopDownController.craftRes` _returnvalue _astop_down_controller))
    (:`==`
      (set `/Game/Gameplay/TopDownController.craftRes` 0 _astop_down_controller :!label _label))
    (:`<`
      (goto _label)))
  (bind _returnvalue_2 (- (`/Game/Gameplay/TopDownController.energy` _astop_down_controller) (`self.requiredEnergy`)))
  (`/Engine/EditorBlueprintResources/StandardMacros.CompareInt` _returnvalue_2
    (:`>`
      (set `/Game/Gameplay/TopDownController.energy` _returnvalue_2 _astop_down_controller :!label _label_2))
    (:`==`
      (goto _label_2))
    (:`<`
      (set `/Game/Gameplay/TopDownController.energy` 0 _astop_down_controller))))

(event `self.UpdateResourcesForPlayer`
  (bind _astop_down_controller (cast `/Game/Gameplay/TopDownController` (`GameplayStatics.GetPlayerController` 0)))
  (`/Game/Gameplay/TopDownController.factoryDidBuild` _astop_down_controller))

(fn `CheckIfCouldBeBuild`
  (returns (couldBeBuilt :type Boolean))
  (bind _astop_down_controller (cast `/Game/Gameplay/TopDownController` (`GameplayStatics.GetPlayerController` 0)))
  (`/Engine/EditorBlueprintResources/StandardMacros.CompareInt` (- (`/Game/Gameplay/TopDownController.craftRes` _astop_down_controller) (`self.requiredCM`))
    (:`>`
      (`/Engine/EditorBlueprintResources/StandardMacros.CompareInt` (- (`/Game/Gameplay/TopDownController.energy` _astop_down_controller) (`self.requiredEnergy`)) :!label _label
        (:`>`
          _)
        (:`==`
          _)
        (:`<`
          (return false))))
    (:`==`
      (goto _label))
    (:`<`
      (return false)))
  (return true))

(fn `UserConstructionScript`)