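; BP_ResourcePile is a finite crafting-resource pile that citizens harvest by standing in it.
; Overlap events count BP_Citizen workers, and each Tick moves one unit per worker from Capacity to the TopDownController's CraftRes, so harvest speed follows frame rate.
; When workers exceed Capacity, CraftRes gains the shortfall instead of the remainder.
; A text render shows Capacity; once depleted, the pile clears CitizensAreBusy and destroys itself.
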(event `self.ReceiveBeginPlay`
  (`TextRenderComponent.K2_SetText` (`self.TextRender`) (`KismetTextLibrary.Conv_IntToText` (`self.capacity`))))

(event `self.ReceiveActorBeginOverlap`
  (params (OtherActor :type "Actor Object Reference"))
  (cast `/Game/Actors/Citizens/BP_Citizen` OtherActor)
  (set `self.workers` (+ (`self.workers`) 1)))

(event `self.ReceiveActorEndOverlap`
  (params (OtherActor :type "Actor Object Reference"))
  (cast `/Game/Actors/Citizens/BP_Citizen` OtherActor)
  (set `self.workers` (- (`self.workers`) 1)))

(event `self.ReceiveTick`
  (params (DeltaSeconds :type "Float (single-precision)"))
  (bind _returnvalue (`GameplayStatics.GetPlayerController` 0))
  (bind _workers (`self.workers`))
  (bind _returnvalue_2 (- (`self.capacity`) _workers))
  (`/Engine/EditorBlueprintResources/StandardMacros.CompareInt` (`self.capacity`)
    (:`>`
      (bind _astop_down_controller (cast `/Game/Gameplay/TopDownController` _returnvalue))
      (`/Engine/EditorBlueprintResources/StandardMacros.CompareInt` _workers
        (:`>`
          (`/Engine/EditorBlueprintResources/StandardMacros.CompareInt` _returnvalue_2
            (:`>`
              (bind _craftres (`/Game/Gameplay/TopDownController.craftRes` _astop_down_controller))
              (set `/Game/Gameplay/TopDownController.craftRes` (+ _craftres _workers) _astop_down_controller :!label _label))
            (:`==`
              (goto _label))
            (:`<`
              (set `/Game/Gameplay/TopDownController.craftRes` (+ _craftres (`KismetMathLibrary.Abs_Int` _returnvalue_2)) _astop_down_controller)))
          (set `self.capacity` _returnvalue_2)
          (`TextRenderComponent.K2_SetText` (`self.TextRender`) (`KismetTextLibrary.Conv_IntToText` (`self.capacity`))))))
    (:`==`
      (bind _astop_down_controller_2 (cast `/Game/Gameplay/TopDownController` _returnvalue :!label _label_2))
      (set `/Game/Gameplay/TopDownController.citizensAreBusy` false _astop_down_controller_2)
      (`self.K2_DestroyActor`))
    (:`<`
      (goto _label_2))))

(fn `UserConstructionScript`)